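; BP_speedUp is a speed boost pickup, shown as a cylinder that yaws a fixed step every Tick, independent of delta time.
; When a BP_Player overlaps its Box, it calls SpeedUpTrigger on that player and hides itself, disabling collision and the Box's overlap events.
; A one-shot ten-second timer then restores visibility and collision, but leaves Box overlap events disabled.
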(event OnComponentBeginOverlap(Box)
  (params (OverlappedComponent :type Primitive%20Component%20Object%20Reference) (OtherActor :type Actor%20Object%20Reference) (OtherComp :type Primitive%20Component%20Object%20Reference) (OtherBodyIndex :type Integer) (bFromSweep :type Boolean) (SweepResult :type Hit%20Result%20Structure%20%28by%20ref%29))
  (bind _asbp_player (Utilities|Casting|CastToBP_Player OtherActor))
  (Default|SpeedUpTrigger _asbp_player)
  (CallFunction|HideActor)
  (Utilities|Time|SetTimerbyEvent (delegate Custom|RespawnActor) 1e+01))

(event Custom|RespawnActor
  (Rendering|SetActorHiddenInGame false)
  (Collision|SetActorEnableCollision true))

(event Custom|HideActor
  (Rendering|SetActorHiddenInGame true)
  (Collision|SetActorEnableCollision false)
  (Variables|/Script/Engine.PrimitiveComponent|SetbGenerateOverlapEvents (Variables|Default|GetBox) false))

(event EventBeginPlay)

(event Collision|EventActorBeginOverlap
  (params (OtherActor :type Actor%20Object%20Reference)))

(event EventTick
  (params (DeltaSeconds :type Float%20%28single-precision%29))
  (bind _cylinder (Variables|Default|GetCylinder))
  (bind _relativerotation (Variables|/Script/Engine.SceneComponent|GetRelativeRotation _cylinder))
  (Transformation|SetRelativeRotation _cylinder (Math|Rotator|MakeRotator (.roll _relativerotation) (.pitch _relativerotation) (+ (.yaw _relativerotation) 2.0)) false false))

(fn ConstructionScript)