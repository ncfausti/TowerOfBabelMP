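; BP_RockSpawn is a spawner actor that continuously emits BP_TagRock actors from its own transform.
; BeginPlay starts an endless Delay loop that spawns a rock every fraction of a second and applies an upward force to its Cube component, with no authority check.
; The server and client rumble events are empty, and the authority switch and Rumble sound nodes are disconnected, so no sound plays.
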(event Custom|SR_PlayRumble)

(event Custom|CL_PlayRumble)

(event EventBeginPlay
  (bind _returnvalue (Game|SpawnActorfromClass "/Game/Blueprints/BP_TagRock.BP_TagRock_C" (Transformation|GetActorTransform) "Undefined" 0 0 :!label _label))
  (Physics|AddForce (Variables|/Game/Blueprints/BP_TagRock.BP_TagRock_C|GetCube _returnvalue) "0, 0,500.000000" "None" false)
  (Utilities|FlowControl|Delay 0.2)
  (goto _label))

(fn ConstructionScript)